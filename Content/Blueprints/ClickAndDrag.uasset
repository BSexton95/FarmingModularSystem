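; Blueprint for mouse click-and-drag of world objects, so far implementing only the pick step.
; While GrabMode is on, a left mouse press deprojects the cursor and runs a complex Visibility line trace with debug drawing.
; A hit component with Movable mobility is stored in GrabbedComponent.
; The physics-simulation check and the mouse release handler lead to no actions, so nothing is dragged or released.
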(event EventBeginPlay)

(event Collision|EventActorBeginOverlap
  (params (OtherActor :type Actor%20Object%20Reference)))

(event EventTick
  (params (DeltaSeconds :type Float%20%28single-precision%29)))

(event Input|MouseEvents|LeftMouseButton
  (params (Key :type Key%20Structure :default "None"))
  (bind _returnvalue (Game|GetPlayerController 0))
  (bind _grabmode (Variables|Default|GetGrabMode))
  (bind (_worldlocation _worlddirection) (Game|Player|ConvertMouseLocationToWorldSpace _returnvalue))
  (:Pressed
    (if _grabmode
      (bind (_outhit _returnvalue_2) (Collision|LineTraceByChannel _worldlocation (+ _worldlocation (* _worlddirection (Math|Float|MakeLiteralFloat 1e+04))) "TraceTypeQuery1" true 0 "ForDuration"))
      (if _returnvalue_2
        (if (== (Variables|/Script/Engine.SceneComponent|GetMobility (.HitComponent (Collision|BreakHitResult _outhit))) (Utilities|Enum|LiteralenumEComponentMobility "Movable"))
          (bind _output_get (Variables|Default|SetGrabbedComponent (.HitComponent (Collision|BreakHitResult _outhit))))
          (if (Physics|IsSimulatingPhysics _output_get "None")
            _)))))
  (:Released
    (if _grabmode
      _)))

(fn ConstructionScript)